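; Fishing rod with a float and hook on two cables, supporting casting, reeling, line locking and reel grabbing.
; Timers pay out or reel in line, syncing cable lengths with physics constraint limits; release casts scale with float velocity.
; In water, the float stops simulating physics, rises and bobs via timeline.
; Tick then redistributes length between cables by slack, lock, reeling and a ground trace below the hook.
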(event OnComponentBeginOverlap(FloatTop)
  (params (OverlappedComponent :type Primitive%20Component%20Object%20Reference) (OtherActor :type Actor%20Object%20Reference) (OtherComp :type Primitive%20Component%20Object%20Reference) (OtherBodyIndex :type Integer) (bFromSweep :type Boolean) (SweepResult :type Hit%20Result%20Structure%20%28by%20ref%29))
  ;[1 1 1] Float Movement
  (Development|PrintString "TopOverlapping" true true "(R=1.000000,G=0.004365,B=0.000000,A=1.000000)" 2e+01)
  (Utilities|Casting|CastToWater OtherActor)
  (Variables|Default|SetIsTopInWater true)
  (if (Variables|Default|GetIsBottomInWater)
    (Variables|Default|SetIsAllInWater true)
    (Utilities|FlowControl|Delay 0.07)
    (Physics|SetSimulatePhysics (Variables|Default|GetFloat) false)
    (Transformation|SetWorldRotation (Variables|Default|GetFloat) "0, 0, 0" false false)
    (Variables|Default|SetIsStartInWater true)
    (Actor|Tick|SetActorTickEnabled true)
    (Utilities|Time|SetTimerbyFunctionName 0 "Float_Up" 0.01 true)))

(event OnComponentBeginOverlap(FloatBottom)
  (params (OverlappedComponent :type Primitive%20Component%20Object%20Reference) (OtherActor :type Actor%20Object%20Reference) (OtherComp :type Primitive%20Component%20Object%20Reference) (OtherBodyIndex :type Integer) (bFromSweep :type Boolean) (SweepResult :type Hit%20Result%20Structure%20%28by%20ref%29))
  ;[1 1 1] Float Movement
  (Development|PrintString "BottomOverlapping" true true "(R=1.000000,G=0.004365,B=0.000000,A=1.000000)" 2e+01)
  (Utilities|Casting|CastToWater OtherActor)
  (Variables|Default|SetIsBottomInWater true)
  (if (Variables|Default|GetIsTopInWater)
    (Variables|Default|SetIsAllInWater true)
    (Utilities|FlowControl|Delay 0.07)
    (Physics|SetSimulatePhysics (Variables|Default|GetFloat) false)
    (Transformation|SetWorldRotation (Variables|Default|GetFloat) "0, 0, 0" false false)
    (Variables|Default|SetIsStartInWater true)
    (Actor|Tick|SetActorTickEnabled true)
    (Utilities|Time|SetTimerbyFunctionName 0 "Float_Up" 0.01 true)))

(event OnComponentEndOverlap(FloatBottom)
  (params (OverlappedComponent :type Primitive%20Component%20Object%20Reference) (OtherActor :type Actor%20Object%20Reference) (OtherComp :type Primitive%20Component%20Object%20Reference) (OtherBodyIndex :type Integer))
  (bind _float (Variables|Default|GetFloat))
  (bind _returnvalue (Transformation|GetWorldLocation _float))
  ;[1 1 1] Float Movement
  (Physics|SetSimulatePhysics (Variables|Default|GetFloat) true)
  (Actor|Tick|SetActorTickEnabled false)
  (Variables|Default|SetIsBottomInWater false)
  (Variables|Default|SetIsTopInWater false)
  (Variables|Default|SetIsAllInWater false)
  (bind _floatmovement (Timeline|T_FloatMovement Stop)
    (:Update
      (Transformation|SetWorldLocation (Variables|Default|GetFloat) (Math|Vector|MakeVector (.x _returnvalue) (.y _returnvalue) (+ _floatmovement (.z _returnvalue))) false false))))

(event OnComponentEndOverlap(FloatStart)
  (params (OverlappedComponent :type Primitive%20Component%20Object%20Reference) (OtherActor :type Actor%20Object%20Reference) (OtherComp :type Primitive%20Component%20Object%20Reference) (OtherBodyIndex :type Integer))
  (bind _float (Variables|Default|GetFloat))
  (bind _returnvalue (Transformation|GetWorldLocation _float))
  ;[1 1 1] Float Movement
  (Utilities|Casting|CastToWater OtherActor)
  (Utilities|Time|ClearTimerbyFunctionName 0 "Float_Up")
  (if (Variables|Default|GetIsStartInWater)
    (Variables|Default|SetIsStartInWater false)
    (bind _floatmovement (Timeline|T_FloatMovement Play)
      (:Update
        (Transformation|SetWorldLocation (Variables|Default|GetFloat) (Math|Vector|MakeVector (.x _returnvalue) (.y _returnvalue) (+ _floatmovement (.z _returnvalue))) false false)))))

(event Custom|E_FloatStopMove
  (bind _float (Variables|Default|GetFloat))
  (bind _returnvalue (Transformation|GetWorldLocation _float))
  ;[1 1 1] Float Movement
  (Development|PrintString "Event On" true true "(R=0.000000,G=0.660000,B=1.000000,A=1.000000)" 1e+01)
  (Physics|SetSimulatePhysics (Variables|Default|GetFloat) true)
  (Actor|Tick|SetActorTickEnabled false)
  (Variables|Default|SetIsBottomInWater false)
  (Variables|Default|SetIsTopInWater false)
  (Variables|Default|SetIsAllInWater false)
  (bind _floatmovement (Timeline|T_FloatMovement Stop)
    (:Update
      (Transformation|SetWorldLocation (Variables|Default|GetFloat) (Math|Vector|MakeVector (.x _returnvalue) (.y _returnvalue) (+ _floatmovement (.z _returnvalue))) false false))))

(event EventRTriggerPressed
  ;[1 1 1] Rod Movement
  (if (Variables|Default|GetIsGrab)
    (Development|PrintString "Grab")
    (elif (Variables|Default|GetIsLock)
      (Development|PrintString "Lock")
      (else
        (Utilities|Time|ClearTimerbyFunctionName 0 "Cable_Set")
        (Utilities|Time|SetTimerbyFunctionName 0 "Reel_In" 0.01 true)))))

(event EventRTriggerReleased
  (bind _pc_rod (Variables|Default|GetPC_Rod))
  ;[1 1 1] Rod Movement
  (Variables|Default|SetIsReeling false)
  (if (not (Variables|Default|GetIsGrab))
    (if (not (Variables|Default|GetIsLock))
      (Utilities|Time|ClearTimerbyFunctionName 0 "Reel_In")
      (Class|PhysicsConstraintComponent|SetLinearXLimit _pc_rod "LCM_Free" 0.0)
      (Class|PhysicsConstraintComponent|SetLinearYLimit _pc_rod "LCM_Free" 0.0)
      (Class|PhysicsConstraintComponent|SetLinearZLimit _pc_rod "LCM_Free" 0.0)
      (Utilities|Time|SetTimerbyFunctionName 0 "Cable_Set" 0.01 true))))

(event EventReleaseReel
  (bind _pc_rod (Variables|Default|GetPC_Rod))
  ;[1 1 1] Rod Movement
  (if (not (Variables|Default|GetIsAllInWater))
    (Variables|Default|SetIsGrab false)
    (if (not (Variables|Default|GetIsLock))
      (Class|PhysicsConstraintComponent|SetLinearXLimit _pc_rod "LCM_Free" 0.0)
      (Class|PhysicsConstraintComponent|SetLinearYLimit _pc_rod "LCM_Free" 0.0)
      (Class|PhysicsConstraintComponent|SetLinearZLimit _pc_rod "LCM_Free" 0.0)
      (if (<= (Variables|/Script/CableComponent.CableComponent|GetCableLength (Variables|Default|GetFloatCable)) 1.0)
        (CallFunction|ReelThrow)
        (else
          (Utilities|Time|SetTimerbyFunctionName 0 "Cable_Set" 0.01 true))))))

(event EventTick
  (params (DeltaSeconds :type Float%20%28single-precision%29))
  ;[1 1 1] Float Movement
  (CallFunction|CableAdjust))

(event EventLTriggerPressed
  (bind _floatcable (Variables|Default|GetFloatCable))
  (bind _pc_rod (Variables|Default|GetPC_Rod))
  (bind _pc_rod_2 (Variables|Default|GetPC_Rod))
  (bind _cablelength (Variables|/Script/CableComponent.CableComponent|GetCableLength _floatcable))
  ;[1 1 1] Rod Movement
  (bind _output_get (Variables|Default|SetIsLock (not (Variables|Default|GetIsLock))))
  (if _output_get
    (Utilities|Time|ClearTimerbyFunctionName 0 "Cable_Set")
    (Utilities|Time|ClearTimerbyFunctionName 0 "Reel_In")
    (Class|PhysicsConstraintComponent|SetLinearXLimit _pc_rod "LCM_Limited" _cablelength)
    (Class|PhysicsConstraintComponent|SetLinearYLimit _pc_rod "LCM_Limited" _cablelength)
    (Class|PhysicsConstraintComponent|SetLinearZLimit _pc_rod "LCM_Limited" _cablelength)
    (else
      (Utilities|Time|ClearTimerbyFunctionName 0 "Cable_Set")
      (Utilities|Time|ClearTimerbyFunctionName 0 "Reel_In")
      (Class|PhysicsConstraintComponent|SetLinearXLimit _pc_rod_2 "LCM_Free" 0.0)
      (Class|PhysicsConstraintComponent|SetLinearYLimit _pc_rod_2 "LCM_Free" 0.0)
      (Class|PhysicsConstraintComponent|SetLinearZLimit _pc_rod_2 "LCM_Free" 0.0)
      (if (not (Variables|Default|GetIsAllInWater))
        (Utilities|Time|SetTimerbyFunctionName 0 "Cable_Set" 0.01 true)))))

(event EventGrabReel
  (bind _floatcable (Variables|Default|GetFloatCable))
  (bind _pc_rod (Variables|Default|GetPC_Rod))
  (bind _cablelength (Variables|/Script/CableComponent.CableComponent|GetCableLength _floatcable))
  ;[1 1 1] Rod Movement
  (if (not (Variables|Default|GetIsAllInWater))
    (Variables|Default|SetIsGrab true)
    (if (not (Variables|Default|GetIsLock))
      (Utilities|Time|ClearTimerbyFunctionName 0 "Cable_Set")
      (Utilities|Time|ClearTimerbyFunctionName 0 "Reel_In")
      (Class|PhysicsConstraintComponent|SetLinearXLimit _pc_rod "LCM_Limited" _cablelength)
      (Class|PhysicsConstraintComponent|SetLinearYLimit _pc_rod "LCM_Limited" _cablelength)
      (Class|PhysicsConstraintComponent|SetLinearZLimit _pc_rod "LCM_Limited" _cablelength)
      (CallFunction|CableSet))))

(fn ConstructionScript)

(fn ReelThrow
  (bind _pc_rod (Variables|Default|GetPC_Rod))
  (bind _output_get (Variables|/Script/CableComponent.CableComponent|SetCableLength (Variables|Default|GetFloatCable) (* (Math|Vector|VectorLength (Transformation|GetComponentVelocity (Variables|Default|GetFloat))) 0.3)))
  (Class|PhysicsConstraintComponent|SetLinearXLimit _pc_rod "LCM_Limited" _output_get)
  (Class|PhysicsConstraintComponent|SetLinearYLimit _pc_rod "LCM_Limited" _output_get)
  (Class|PhysicsConstraintComponent|SetLinearZLimit _pc_rod "LCM_Limited" _output_get))

(fn Reelin
  (bind _hookcable (Variables|Default|GetHookCable))
  (bind _float (Variables|Default|GetFloat))
  (bind _floatcable (Variables|Default|GetFloatCable))
  (bind _pc_rod (Variables|Default|GetPC_Rod))
  (bind _pc_sub (Variables|Default|GetPC_Sub))
  (bind _pc_sub_2 (Variables|Default|GetPC_Sub))
  (bind _pc_rod_2 (Variables|Default|GetPC_Rod))
  (bind _pc_rod_3 (Variables|Default|GetPC_Rod))
  (bind _returnvalue (Transformation|GetWorldLocation _float))
  (bind _returnvalue_2 (Transformation|GetWorldLocation _pc_rod))
  (bind _returnvalue_3 (Transformation|GetWorldLocation _pc_sub))
  (bind _returnvalue_4 (Math|Rotator|FindLookatRotation _returnvalue_3 _returnvalue_2))
  (bind _returnvalue_5 (Math|Vector|GetForwardVector _returnvalue_4))
  (Variables|Default|SetIsLock false)
  (if (> (Variables|/Script/CableComponent.CableComponent|GetCableLength (Variables|Default|GetFloatCable)) 1.0)
    (if (Variables|Default|GetIsAllInWater)
      (Variables|Default|SetIsReeling true)
      (if (> (Variables|/Script/CableComponent.CableComponent|GetCableLength (Variables|Default|GetHookCable)) 2.0)
        (Development|PrintString "ReelUp")
        (bind _output_get (Variables|/Script/CableComponent.CableComponent|SetCableLength _hookcable (- (Variables|/Script/CableComponent.CableComponent|GetCableLength _hookcable) 0.3)))
        (Class|PhysicsConstraintComponent|SetLinearXLimit _pc_sub_2 "LCM_Limited" _output_get)
        (Class|PhysicsConstraintComponent|SetLinearYLimit _pc_sub_2 "LCM_Limited" _output_get)
        (Class|PhysicsConstraintComponent|SetLinearZLimit _pc_sub_2 "LCM_Limited" _output_get)
        (else
          (Transformation|SetWorldLocation (Variables|Default|GetFloat) (Math|Vector|MakeVector (+ (* (.x _returnvalue_5) 1.0) (.x _returnvalue)) (+ (* (.y _returnvalue_5) 1.0) (.y _returnvalue)) (.z _returnvalue)) false false)
          (Class|PhysicsConstraintComponent|SetLinearXLimit _pc_rod_2 "LCM_Limited" (Variables|/Script/CableComponent.CableComponent|GetCableLength (Variables|Default|GetFloatCable)))
          (Class|PhysicsConstraintComponent|SetLinearYLimit _pc_rod_2 "LCM_Limited" (Variables|/Script/CableComponent.CableComponent|GetCableLength (Variables|Default|GetFloatCable)))
          (Class|PhysicsConstraintComponent|SetLinearZLimit _pc_rod_2 "LCM_Limited" (Variables|/Script/CableComponent.CableComponent|GetCableLength (Variables|Default|GetFloatCable)))))
      (else
        (bind _output_get_2 (Variables|/Script/CableComponent.CableComponent|SetCableLength _floatcable (- (Variables|/Script/CableComponent.CableComponent|GetCableLength _floatcable) 0.7)))
        (Class|PhysicsConstraintComponent|SetLinearXLimit _pc_rod_3 "LCM_Limited" _output_get_2)
        (Class|PhysicsConstraintComponent|SetLinearYLimit _pc_rod_3 "LCM_Limited" _output_get_2)
        (Class|PhysicsConstraintComponent|SetLinearZLimit _pc_rod_3 "LCM_Limited" _output_get_2)))))

(fn FloatUp
  (Transformation|AddWorldOffset (Variables|Default|GetFloat) (Math|Vector|MakeVector 0.0 0.0 0.1) false false))

(fn CableAdjust
  (bind _floatcable (Variables|Default|GetFloatCable))
  (bind _pc_rod (Variables|Default|GetPC_Rod))
  (bind _pc_sub (Variables|Default|GetPC_Sub))
  (bind _hook (Variables|Default|GetHook))
  (bind _pc_rod_2 (Variables|Default|GetPC_Rod))
  (bind _float (Variables|Default|GetFloat))
  (bind _pc_sub_2 (Variables|Default|GetPC_Sub))
  (bind _pc_rod_3 (Variables|Default|GetPC_Rod))
  (bind _pc_sub_3 (Variables|Default|GetPC_Sub))
  (bind _hookcable (Variables|Default|GetHookCable))
  (bind _pc_rod_4 (Variables|Default|GetPC_Rod))
  (bind _hook_2 (Variables|Default|GetHook))
  (bind _floatcable_2 (Variables|Default|GetFloatCable))
  (bind _pc_rod_5 (Variables|Default|GetPC_Rod))
  (bind _pc_sub_4 (Variables|Default|GetPC_Sub))
  (bind _pc_rod_6 (Variables|Default|GetPC_Rod))
  (bind _pc_rod_7 (Variables|Default|GetPC_Rod))
  (bind _pc_sub_5 (Variables|Default|GetPC_Sub))
  (bind _pc_sub_6 (Variables|Default|GetPC_Sub))
  (bind _pc_rod_8 (Variables|Default|GetPC_Rod))
  (bind _pc_rod_9 (Variables|Default|GetPC_Rod))
  (bind _pc_sub_7 (Variables|Default|GetPC_Sub))
  (bind _returnvalue (Transformation|GetWorldLocation _hook))
  (bind _returnvalue_2 (Transformation|GetWorldLocation _float))
  (bind _returnvalue_3 (Transformation|GetWorldLocation _hook_2))
  (bind _returnvalue_4 (Transformation|GetWorldLocation _pc_rod_7))
  (bind _returnvalue_5 (Transformation|GetWorldLocation _pc_sub_5))
  (bind _returnvalue_6 (Math|Rotator|FindLookatRotation _returnvalue_5 _returnvalue_4))
  (bind _returnvalue_7 (Math|Vector|GetForwardVector _returnvalue_6))
  (Variables|Default|SetDistanceRodToFloat (Math|Float|Absolute(Float) (Math|Vector|Distance(Vector) (Transformation|GetWorldLocation (Variables|Default|GetPC_Rod)) (Transformation|GetWorldLocation (Variables|Default|GetPC_Sub)))))
  (Variables|Default|SetDistanceFloatToHook (Math|Float|Absolute(Float) (Math|Vector|Distance(Vector) (Transformation|GetWorldLocation (Variables|Default|GetFloat)) (Transformation|GetWorldLocation (Variables|Default|GetHook)))))
  ;[1 1 1] Cable - Distance
  (Variables|Default|SetCableAdjustFloat (- (Variables|/Script/CableComponent.CableComponent|GetCableLength (Variables|Default|GetFloatCable)) (Variables|Default|GetDistanceRodToFloat)))
  ;[1 1 1] 줄이 느슨한가, 팽팽한가
  (if (> (Variables|/Script/CableComponent.CableComponent|GetCableLength (Variables|Default|GetFloatCable)) (Variables|Default|GetDistanceRodToFloat))
    (bind _outhit (Collision|LineTraceByChannel (Transformation|GetWorldLocation (Variables|Default|GetHook)) (Math|Vector|MakeVector (.x _returnvalue_3) (.y _returnvalue_3) (- (.z _returnvalue_3) 1e+02)) "TraceTypeQuery1" false 0 "None"))
    ;[1 1 1] 허공에 있는가
    (if (> (Math|Vector|Distance(Vector) (.location _outhit) (Transformation|GetWorldLocation (Variables|Default|GetHook))) 1e+01)
      ;[1 1 1] 땅에 안닿았을때, 잠겨 있는가
      (if (Variables|Default|GetIsLock)
        (Utilities|FlowControl|Sequence :!label _label
          (:then_0
            ;[1 1 1] 플로트 케이블 팽팽하게
            ;;[1 1 1] 살짝 오류
            (bind _output_get (Variables|/Script/CableComponent.CableComponent|SetCableLength (Variables|Default|GetFloatCable) (Variables|Default|GetDistanceRodToFloat)))
            (Class|PhysicsConstraintComponent|SetLinearXLimit _pc_rod_6 "LCM_Limited" _output_get)
            (Class|PhysicsConstraintComponent|SetLinearYLimit _pc_rod_6 "LCM_Limited" _output_get)
            (Class|PhysicsConstraintComponent|SetLinearZLimit _pc_rod_6 "LCM_Limited" _output_get))
          (:then_1
            (bind _output_get_2 (Variables|/Script/CableComponent.CableComponent|SetCableLength (Variables|Default|GetHookCable) (+ (Variables|Default|GetCableAdjustFloat) (Variables|Default|GetDistanceFloatToHook))))
            (Class|PhysicsConstraintComponent|SetLinearXLimit _pc_sub_4 "LCM_Limited" _output_get_2)
            (Class|PhysicsConstraintComponent|SetLinearYLimit _pc_sub_4 "LCM_Limited" _output_get_2)
            (Class|PhysicsConstraintComponent|SetLinearZLimit _pc_sub_4 "LCM_Limited" _output_get_2)))
        (elif (Variables|Default|GetIsReeling)
          (goto _label)
          (else
            (Utilities|FlowControl|Sequence
              (:then_0
                (bind _output_get_3 (Variables|/Script/CableComponent.CableComponent|SetCableLength _floatcable_2 (Variables|/Script/CableComponent.CableComponent|GetCableLength _floatcable_2)))
                (Class|PhysicsConstraintComponent|SetLinearXLimit _pc_rod_3 "LCM_Limited" _output_get_3)
                (Class|PhysicsConstraintComponent|SetLinearYLimit _pc_rod_3 "LCM_Limited" _output_get_3)
                (Class|PhysicsConstraintComponent|SetLinearZLimit _pc_rod_3 "LCM_Limited" _output_get_3))
              (:then_1
                (bind _output_get_4 (Variables|/Script/CableComponent.CableComponent|SetCableLength (Variables|Default|GetHookCable) (+ (Variables|Default|GetCableAdjustFloat) (Variables|Default|GetDistanceFloatToHook))))
                (Class|PhysicsConstraintComponent|SetLinearXLimit _pc_sub_2 "LCM_Limited" _output_get_4)
                (Class|PhysicsConstraintComponent|SetLinearYLimit _pc_sub_2 "LCM_Limited" _output_get_4)
                (Class|PhysicsConstraintComponent|SetLinearZLimit _pc_sub_2 "LCM_Limited" _output_get_4))))))
      (else
        ;[1 1 1] 땅에 닿았을때, 잠겨있는가
        (if (Variables|Default|GetIsLock)
          (Class|PhysicsConstraintComponent|SetLinearXLimit _pc_rod_5 "LCM_Limited" (Variables|/Script/CableComponent.CableComponent|GetCableLength (Variables|Default|GetFloatCable)) :!label _label_2)
          (Class|PhysicsConstraintComponent|SetLinearYLimit _pc_rod_5 "LCM_Limited" (Variables|/Script/CableComponent.CableComponent|GetCableLength (Variables|Default|GetFloatCable)))
          (Class|PhysicsConstraintComponent|SetLinearZLimit _pc_rod_5 "LCM_Limited" (Variables|/Script/CableComponent.CableComponent|GetCableLength (Variables|Default|GetFloatCable)))
          (elif (Variables|Default|GetIsReeling)
            (goto _label_2)
            (else
              (Utilities|FlowControl|Sequence
                (:then_0
                  ;[1 1 1] Float Cable 그대로
                  (Class|PhysicsConstraintComponent|SetLinearXLimit _pc_rod_8 "LCM_Free" (Variables|/Script/CableComponent.CableComponent|GetCableLength (Variables|Default|GetFloatCable)))
                  (Class|PhysicsConstraintComponent|SetLinearYLimit _pc_rod_8 "LCM_Free" (Variables|/Script/CableComponent.CableComponent|GetCableLength (Variables|Default|GetFloatCable)))
                  (Class|PhysicsConstraintComponent|SetLinearZLimit _pc_rod_8 "LCM_Free" (Variables|/Script/CableComponent.CableComponent|GetCableLength (Variables|Default|GetFloatCable))))
                (:then_1
                  (Variables|/Script/CableComponent.CableComponent|SetCableLength (Variables|Default|GetHookCable) (Variables|Default|GetDistanceFloatToHook))
                  (Class|PhysicsConstraintComponent|SetLinearXLimit _pc_sub_7 "LCM_Free" 0.0)
                  (Class|PhysicsConstraintComponent|SetLinearYLimit _pc_sub_7 "LCM_Free" 0.0)
                  (Class|PhysicsConstraintComponent|SetLinearZLimit _pc_sub_7 "LCM_Free" 0.0))))))))
    (elif (Variables|Default|GetIsLock)
      ;[1 1 1] Hook Cable > 2
      (if (> (Variables|/Script/CableComponent.CableComponent|GetCableLength (Variables|Default|GetHookCable)) 2.0) :!label _label_3
        (bind _outhit_2 (Collision|LineTraceByChannel (Transformation|GetWorldLocation (Variables|Default|GetHook)) (Math|Vector|MakeVector (.x _returnvalue) (.y _returnvalue) (- (.z _returnvalue) 1e+02)) "TraceTypeQuery1" false 0 "None"))
        ;[1 1 1] 땅에 닿았는가
        (if (> (Math|Vector|Distance(Vector) (.location _outhit_2) (Transformation|GetWorldLocation (Variables|Default|GetHook))) 1e+01)
          (Utilities|FlowControl|Sequence
            (:then_0
              ;[1 1 1] 플로트 케이블 팽팽하게
              ;;[1 1 1] 살짝 오류
              (bind _output_get_5 (Variables|/Script/CableComponent.CableComponent|SetCableLength (Variables|Default|GetFloatCable) (Variables|Default|GetDistanceRodToFloat)))
              (Class|PhysicsConstraintComponent|SetLinearXLimit _pc_rod_2 "LCM_Limited" _output_get_5)
              (Class|PhysicsConstraintComponent|SetLinearYLimit _pc_rod_2 "LCM_Limited" _output_get_5)
              (Class|PhysicsConstraintComponent|SetLinearZLimit _pc_rod_2 "LCM_Limited" _output_get_5))
            (:then_1
              (bind _output_get_6 (Variables|/Script/CableComponent.CableComponent|SetCableLength _hookcable (+ (Variables|Default|GetCableAdjustFloat) (Variables|/Script/CableComponent.CableComponent|GetCableLength _hookcable))))
              (Class|PhysicsConstraintComponent|SetLinearXLimit _pc_sub_3 "LCM_Limited" _output_get_6)
              (Class|PhysicsConstraintComponent|SetLinearYLimit _pc_sub_3 "LCM_Limited" _output_get_6)
              (Class|PhysicsConstraintComponent|SetLinearZLimit _pc_sub_3 "LCM_Limited" _output_get_6)))
          (else
            (Utilities|FlowControl|Sequence
              (:then_0
                ;[1 1 1] 플로트 케이블 팽팽하게
                (bind _output_get_7 (Variables|/Script/CableComponent.CableComponent|SetCableLength (Variables|Default|GetFloatCable) (Variables|Default|GetDistanceRodToFloat)))
                (Class|PhysicsConstraintComponent|SetLinearXLimit _pc_rod "LCM_Limited" _output_get_7)
                (Class|PhysicsConstraintComponent|SetLinearYLimit _pc_rod "LCM_Limited" _output_get_7)
                (Class|PhysicsConstraintComponent|SetLinearZLimit _pc_rod "LCM_Limited" _output_get_7))
              (:then_1
                (bind _output_get_8 (Variables|/Script/CableComponent.CableComponent|SetCableLength (Variables|Default|GetHookCable) (+ (Variables|Default|GetCableAdjustFloat) (Variables|Default|GetDistanceFloatToHook))))
                (Class|PhysicsConstraintComponent|SetLinearXLimit _pc_sub "LCM_Limited" _output_get_8)
                (Class|PhysicsConstraintComponent|SetLinearYLimit _pc_sub "LCM_Limited" _output_get_8)
                (Class|PhysicsConstraintComponent|SetLinearZLimit _pc_sub "LCM_Limited" _output_get_8)))))
        (elif (> (Variables|Default|GetDistanceRodToFloat) (- (.z (Transformation|GetWorldLocation (Variables|Default|GetPC_Rod))) (.z (Transformation|GetWorldLocation (Variables|Default|GetPC_Sub)))))
          (Transformation|SetWorldLocation (Variables|Default|GetFloat) (Math|Vector|MakeVector (+ (* (.x _returnvalue_7) 1.0) (.x _returnvalue_2)) (+ (* (.y _returnvalue_7) 1.0) (.y _returnvalue_2)) (.z _returnvalue_2)) false false)
          (Class|PhysicsConstraintComponent|SetLinearXLimit _pc_rod_9 "LCM_Limited" (Variables|/Script/CableComponent.CableComponent|GetCableLength (Variables|Default|GetFloatCable)))
          (Class|PhysicsConstraintComponent|SetLinearYLimit _pc_rod_9 "LCM_Limited" (Variables|/Script/CableComponent.CableComponent|GetCableLength (Variables|Default|GetFloatCable)))
          (Class|PhysicsConstraintComponent|SetLinearZLimit _pc_rod_9 "LCM_Limited" (Variables|/Script/CableComponent.CableComponent|GetCableLength (Variables|Default|GetFloatCable)))
          (else
            (Development|PrintString "EscapeWater" true true "(R=0.000000,G=0.660000,B=1.000000,A=1.000000)" 1e+01)
            ;[1 1 1] 튀어오름
            (CallFunction|EFloatStopMove))))
      (elif (Variables|Default|GetIsReeling)
        (goto _label_3)
        (else
          (Utilities|FlowControl|Sequence
            (:then_0
              (bind _output_get_9 (Variables|/Script/CableComponent.CableComponent|SetCableLength _floatcable (Variables|/Script/CableComponent.CableComponent|GetCableLength _floatcable)))
              (Class|PhysicsConstraintComponent|SetLinearXLimit _pc_rod_4 "LCM_Limited" _output_get_9)
              (Class|PhysicsConstraintComponent|SetLinearYLimit _pc_rod_4 "LCM_Limited" _output_get_9)
              (Class|PhysicsConstraintComponent|SetLinearZLimit _pc_rod_4 "LCM_Limited" _output_get_9))
            (:then_1
              (Variables|/Script/CableComponent.CableComponent|SetCableLength (Variables|Default|GetHookCable) (+ (Variables|Default|GetCableAdjustFloat) (Variables|Default|GetDistanceFloatToHook)))
              (Class|PhysicsConstraintComponent|SetLinearXLimit _pc_sub_6 "LCM_Free" 0.0)
              (Class|PhysicsConstraintComponent|SetLinearYLimit _pc_sub_6 "LCM_Free" 0.0)
              (Class|PhysicsConstraintComponent|SetLinearZLimit _pc_sub_6 "LCM_Free" 0.0))))))))

(fn CableSet
  (Variables|/Script/CableComponent.CableComponent|SetCableLength (Variables|Default|GetFloatCable) (Math|Float|Absolute(Float) (Math|Vector|Distance(Vector) (Transformation|GetWorldLocation (Variables|Default|GetPC_Rod)) (Transformation|GetWorldLocation (Variables|Default|GetPC_Sub))))))